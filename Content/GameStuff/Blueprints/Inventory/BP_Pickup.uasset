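; BP_Pickup is a world pickup that adds an item class and amount to the player's inventory on touch.
; The sphere overlap calls AddItem on CH_Player's Inventory, keeping any remainder in the pickup or destroying it once everything is taken.
; The construction script reads the item class defaults to show either a skeletal or static mesh, leaving both components untouched for specimen items.
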(event OnComponentBeginOverlap(Sphere)
  (params (OverlappedComponent :type Primitive%20Component%20Object%20Reference) (OtherActor :type Actor%20Object%20Reference) (OtherComp :type Primitive%20Component%20Object%20Reference) (OtherBodyIndex :type Integer) (bFromSweep :type Boolean) (SweepResult :type Hit%20Result%20Structure%20%28by%20ref%29))
  (bind _asch_player (Utilities|Casting|CastToCH_Player OtherActor))
  (Utilities|IsValid (Variables|/Game/GameStuff/Blueprints/Characters/CH_Player.CH_Player_C|GetInventory _asch_player)
    (:Is%20Valid
      (bind (_success _remaining) (Default|AddItem (Variables|/Game/GameStuff/Blueprints/Characters/CH_Player.CH_Player_C|GetInventory _asch_player) (Variables|Default|GetItemToAdd) (Variables|Default|GetAmount)))
      (if _success
        (if (> _remaining 0)
          (Variables|Default|SetAmount _remaining)
          (else
            (Actor|DestroyActor)))))))

(event EventBeginPlay)

(event Collision|EventActorBeginOverlap
  (params (OtherActor :type Actor%20Object%20Reference)))

(event EventTick
  (params (DeltaSeconds :type Float%20%28single-precision%29)))

(fn ConstructionScript
  (bind _itemtoadd (Variables|Default|GetItemToAdd))
  (bind _skeletalmesh (Variables|Default|GetSkeletalMesh))
  (bind _staticmesh (Variables|Default|GetStaticMesh))
  (bind _iteminfo (Utilities|GetClassDefaults _itemtoadd))
  (bind (_name _description _icon _canbeused_ _usedtext _canbestacked_ _itemtype _isskeletal_ _skeletalmesh_2 _staticmesh_2 _isspecimen_) (Utilities|Struct|BreakS_ItemInfo _iteminfo))
  (if (not _isspecimen_)
    (Rendering|SetVisibility _skeletalmesh false false)
    (Rendering|SetVisibility _staticmesh false false)
    (if _isskeletal_
      (Rendering|SetVisibility _staticmesh false false)
      (Class|SkinnedMeshComponent|SetSkeletalMesh _skeletalmesh _skeletalmesh_2 true)
      (Rendering|SetVisibility _skeletalmesh true false)
      (else
        (Rendering|SetVisibility _skeletalmesh false false)
        (Components|StaticMesh|SetStaticMesh _staticmesh _staticmesh_2)
        (Rendering|SetVisibility _staticmesh true false)))))
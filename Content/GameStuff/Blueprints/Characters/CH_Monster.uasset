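; Monster enemy character that wanders to random reachable points and attacks the player in melee.
; Pawn sensing switches it to chasing the player with AIMoveTo, playing an attack montage once within range.
; A separate Attack event, not called in this graph, sphere-traces forward to damage the player, then attacks again or resumes the chase by distance.
; Random sound playback logic is present but disconnected.
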(event OnSeePawn(PawnSensing)
  (params (Pawn :type Pawn%20Object%20Reference))
  (bind _player (Variables|Default|GetPlayer))
  (if (== Pawn _player)
    (CallFunction|MovetoPlayer _player)))

(event Custom|Patrol
  (AI|AIMoveTo self (.RandomLocation (AI|Navigation|GetRandomReachablePointinRadius (Transformation|GetActorLocation) 1e+03 0 0)) 0 5e+01 false
    (:OnSuccess
      (Utilities|FlowControl|Delay 0.2)
      (if (< (Transformation|GetDistanceTo self (Variables|Default|GetPlayer)) 2.5e+02) :!label _label
        (CallFunction|LaunchAttack)
        (Utilities|FlowControl|Delay 2.0)
        (goto _label)
        (else
          (CallFunction|Patrol))))))

(event Custom|MoveToPlayer
  (params (Player :type CH%20Player%20Object%20Reference))
  (AI|AIMoveTo self "0, 0, 0" Player 2.5e+02 false
    (:OnSuccess
      (Utilities|FlowControl|Delay 0.2)
      (if (< (Transformation|GetDistanceTo self Player) 2.5e+02)
        (CallFunction|LaunchAttack)
        (else
          (CallFunction|MovetoPlayer Player))))))

(event Custom|Attack
  (bind _returnvalue (Transformation|GetActorLocation))
  (bind (_outhits _returnvalue_2) (Collision|MultiSphereTraceForObjects _returnvalue (+ _returnvalue (* (Transformation|GetActorForwardVector) 2.5e+02)) 25.0 (Utilities|Array|MakeArray "ObjectTypeQuery3") false (Utilities|Array|MakeArray self) "None"))
  (if _returnvalue_2
    (for _array_element _outhits
      (bind _asch_player (Utilities|Casting|CastToCH_Player (.HitActor (Collision|BreakHitResult _array_element))))
      (Game|Damage|ApplyDamage _asch_player 15.0 0 0)
      (if (< (Transformation|GetDistanceTo self _asch_player) 1e+03)
        (CallFunction|LaunchAttack)
        (else
          (CallFunction|MovetoPlayer _asch_player))))))

(event Custom|LaunchAttack
  (Animation|StopAnimMontage 0)
  (Animation|PlayAnimMontage "/Game/GameStuff/Models/Miner/Animations/Monster_Attack.Monster_Attack" 1.0 "None"))

(event EventBeginPlay
  (bind _asch_player (Utilities|Casting|CastToCH_Player (Game|GetPlayerCharacter 0)))
  (Variables|Default|SetPlayer _asch_player)
  (CallFunction|Patrol))

(event Collision|EventActorBeginOverlap
  (params (OtherActor :type Actor%20Object%20Reference)))

(event EventTick
  (params (DeltaSeconds :type Float%20%28single-precision%29)))

(fn ConstructionScript)
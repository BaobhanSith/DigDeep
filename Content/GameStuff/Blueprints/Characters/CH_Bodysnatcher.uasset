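; CH_Bodysnatcher is a character that chases the player once its pawn sensing sees them.
; A sighting plays a random sound from Sounds at its location, gated by HasPlayedSound, and calls MoveToPlayer.
; MoveToPlayer issues an AI move toward the player, then after a delay clears the sound flag and calls itself, so the pursuit repeats without further sightings.
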(event OnSeePawn(PawnSensing)
  (params (Pawn :type Pawn%20Object%20Reference))
  (bind _sounds (Variables|Default|GetSounds))
  (bind _asch_player (Utilities|Casting|CastToCH_Player Pawn))
  (Utilities|FlowControl|Sequence
    (:then_0
      (if (not (Variables|Default|GetHasPlayedSound?))
        (Audio|PlaySoundatLocation (Utilities|Array|Get(acopy) _sounds (Math|Random|RandomIntegerinRange 0 (- (Utilities|Array|Length _sounds) 1))) (Transformation|GetActorLocation) "0, 0, 0" 1.0 1.0 0.0 0 0 0)
        (Variables|Default|SetHasPlayedSound? true)))
    (:then_1
      (CallFunction|MovetoPlayer _asch_player))))

(event Custom|MoveToPlayer
  (params (Player :type CH%20Player%20Object%20Reference))
  (AI|AIMoveTo self "0, 0, 0" Player 5.0 false
    (:then
      _)
    (:OnSuccess
      _)
    (:OnFail
      _))
  (Utilities|FlowControl|Delay 2.0)
  (Variables|Default|SetHasPlayedSound? false)
  (CallFunction|MovetoPlayer Player))

(event EventBeginPlay)

(event Collision|EventActorBeginOverlap
  (params (OtherActor :type Actor%20Object%20Reference)))

(event EventTick
  (params (DeltaSeconds :type Float%20%28single-precision%29)))

(fn ConstructionScript)
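; Test AI monster character that senses the player and performs a melee attack, with its state shared through the AI controller's Blackboard.
; BeginPlay publishes the attack range, and perception updates write the player's visibility, location and reference for AI logic to use.
; LaunchAttack restarts the attack montage.
; A separate Attack event sphere-traces forward for pawns and damages players hit, leaving persistent debug drawing.
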(event OnTargetPerceptionUpdated(AIPerception)
  (params (Actor :type Actor%20Object%20Reference) (Stimulus :type AI%20Stimulus%20Structure))
  (bind _self self)
  (bind _returnvalue (AI|GetAIController _self))
  (bind _returnvalue_2 (AI|GetBlackboard _returnvalue))
  (bind _asch_player (Utilities|Casting|CastToCH_Player Actor))
  (AI|Components|Blackboard|SetValueasBool _returnvalue_2 (Utilities|Name|MakeLiteralName "SeePlayer") (.bsuccessfullysensed Stimulus))
  (AI|Components|Blackboard|SetValueasVector _returnvalue_2 (Utilities|Name|MakeLiteralName "PlayerLocation") (Transformation|GetActorLocation _asch_player))
  (AI|Components|Blackboard|SetValueasObject _returnvalue_2 (Utilities|Name|MakeLiteralName "Player") _asch_player))

(event Custom|Attack
  (bind _returnvalue (Transformation|GetActorLocation))
  (bind (_outhits _returnvalue_2) (Collision|MultiSphereTraceForObjects _returnvalue (+ _returnvalue (* (Transformation|GetActorForwardVector) (Variables|Default|GetAttackRange))) 25.0 (Utilities|Array|MakeArray "ObjectTypeQuery3") false (Utilities|Array|MakeArray self) "Persistent"))
  (if _returnvalue_2
    (for _array_element _outhits
      (bind _asch_player (Utilities|Casting|CastToCH_Player (.HitActor (Collision|BreakHitResult _array_element))))
      (Game|Damage|ApplyDamage _asch_player 15.0 0 0))))

(event Custom|LaunchAttack
  (Animation|StopAnimMontage 0)
  (Animation|PlayAnimMontage "/Game/GameStuff/Models/Miner/Animations/Monster_Attack.Monster_Attack" 1.0 "None"))

(event EventBeginPlay
  (AI|Components|Blackboard|SetValueasFloat (AI|GetBlackboard (AI|GetAIController self)) (Utilities|Name|MakeLiteralName "AttackDistance") (Variables|Default|GetAttackRange)))

(event Collision|EventActorBeginOverlap
  (params (OtherActor :type Actor%20Object%20Reference)))

(event EventTick
  (params (DeltaSeconds :type Float%20%28single-precision%29)))

(fn ConstructionScript)
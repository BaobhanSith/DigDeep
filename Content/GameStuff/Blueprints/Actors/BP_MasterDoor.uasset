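; Configurable master door actor that the player opens by interacting, with variants for door type, lock side and required item.
; The construction script picks mesh and anim class, enables unlock-volume collision and shows slime on acid doors.
; Interaction checks the player's side and items on first use, then makes the box overlap-only, sets IsOpening and, after a per-type delay, marks it opened and hides slime.
; Montage playback is disconnected.
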(event OnComponentBeginOverlap(Box)
  (params (OverlappedComponent :type Primitive%20Component%20Object%20Reference) (OtherActor :type Actor%20Object%20Reference) (OtherComp :type Primitive%20Component%20Object%20Reference) (OtherBodyIndex :type Integer) (bFromSweep :type Boolean) (SweepResult :type Hit%20Result%20Structure%20%28by%20ref%29)))

(event Custom|OnInteractWith
  (params (Player :type CH%20Player%20Object%20Reference))
  (bind _backunlock (Variables|Default|GetBackUnlock))
  (bind _frontunlock (Variables|Default|GetFrontUnlock))
  (bind _capsulecomponent (Variables|/Script/Engine.Character|GetCapsuleComponent Player))
  (bind _returnvalue (Class|PrimitiveComponent|IsOverlappingComponent _backunlock _capsulecomponent))
  (bind _returnvalue_2 (Class|PrimitiveComponent|IsOverlappingComponent _frontunlock _capsulecomponent))
  (if (Variables|Default|GetHasBeenOpened?)
    (Collision|SetCollisionProfileName (Variables|Default|GetBox) "OverlapAllDynamic" :!class /Script/Engine.PrimitiveComponent :!label _label)
    (Variables|Default|SetIsOpening? true)
    (switch Utilities|FlowControl|Switch|SwitchonE_DoorTypes (Variables|Default|GetDoorType)
      (:NewEnumerator1
        (Utilities|FlowControl|Delay 1.0))
      (:NewEnumerator2
        (Utilities|FlowControl|Delay 1.5))
      (:NewEnumerator3
        (Utilities|FlowControl|Delay 1.0))
      (:NewEnumerator4
        (Utilities|FlowControl|Delay 2.0)))
    (Variables|Default|SetHasBeenOpened? true)
    (if (Variables|Default|GetIsAcidDoor?)
      (Rendering|SetVisibility (Variables|Default|GetSlime) false false))
    (else
      (switch Utilities|FlowControl|Switch|SwitchonE_LockType (Variables|Default|GetLockType)
        (:NewEnumerator0
          (switch Utilities|FlowControl|Switch|SwitchonE_OpenTypes (Variables|Default|GetOpenType) :!label _label_2
            (:NewEnumerator0
              (goto _label))
            (:NewEnumerator1
              (if (Variables|/Game/GameStuff/Blueprints/Characters/CH_Player.CH_Player_C|GetHasWrench? Player)
                (goto _label)))
            (:NewEnumerator2
              (if (> (Utilities|Array|Length (Variables|/Game/GameStuff/Blueprints/Characters/CH_Player.CH_Player_C|GetAcids Player)) 0)
                (goto _label)))
            (:NewEnumerator3
              (if (Variables|/Game/GameStuff/Blueprints/Characters/CH_Player.CH_Player_C|GetHasCode? Player)
                (goto _label)))
            (:NewEnumerator4
              (goto _label))
            (:NewEnumerator5
              (if (Variables|/Game/GameStuff/Blueprints/Characters/CH_Player.CH_Player_C|GetHasKeycard? Player)
                (goto _label)))))
        (:NewEnumerator1
          (if _returnvalue_2
            (goto _label_2)))
        (:NewEnumerator2
          (if _returnvalue
            (goto _label_2)))
        (:NewEnumerator3
          (if (or _returnvalue_2 _returnvalue)
            (goto _label_2)))))))

(fn ConstructionScript
  (bind _skeletalmesh (Variables|Default|GetSkeletalMesh))
  (bind _frontunlock (Variables|Default|GetFrontUnlock))
  (bind _backunlock (Variables|Default|GetBackUnlock))
  (switch Utilities|FlowControl|Switch|SwitchonE_DoorTypes (Variables|Default|GetDoorType)
    (:NewEnumerator1
      (Class|SkinnedMeshComponent|SetSkeletalMesh _skeletalmesh "/Game/GameStuff/Models/Doors/Models/Door_Standard_01.Door_Standard_01" true)
      (Class|SkeletalMeshComponent|SetAnimClass _skeletalmesh "/Game/GameStuff/Models/Doors/Animations/Standard/DoorStandard_AnimBP.DoorStandard_AnimBP_C"))
    (:NewEnumerator2
      (Class|SkinnedMeshComponent|SetSkeletalMesh _skeletalmesh "/Game/GameStuff/Models/Doors/Models/Door_Standard_Bolted_01.Door_Standard_Bolted_01" true)
      (Class|SkeletalMeshComponent|SetAnimClass _skeletalmesh "/Game/GameStuff/Models/Doors/Animations/Bolted/DoorBolted_AnimBP.DoorBolted_AnimBP_C"))
    (:NewEnumerator3
      (Class|SkinnedMeshComponent|SetSkeletalMesh _skeletalmesh "/Game/GameStuff/Models/Doors/Models/Door_Standard_Keypad_01.Door_Standard_Keypad_01" true)
      (Class|SkeletalMeshComponent|SetAnimClass _skeletalmesh "/Game/GameStuff/Models/Doors/Animations/Keypad/DoorKeypad_AnimBP.DoorKeypad_AnimBP_C"))
    (:NewEnumerator4
      (Class|SkinnedMeshComponent|SetSkeletalMesh _skeletalmesh "/Game/GameStuff/Models/Doors/Models/Door_Standard_01.Door_Standard_01" true)
      (Class|SkeletalMeshComponent|SetAnimClass _skeletalmesh "/Game/GameStuff/Models/Doors/Animations/Broken/DoorBroken_AnimBP.DoorBroken_AnimBP_C")))
  (switch Utilities|FlowControl|Switch|SwitchonE_LockType (Variables|Default|GetLockType)
    (:NewEnumerator0
      (Collision|SetCollisionEnabled _backunlock "QueryAndPhysics")
      (Collision|SetCollisionEnabled _frontunlock "QueryAndPhysics"))
    (:NewEnumerator1
      (Collision|SetCollisionEnabled _frontunlock "QueryAndPhysics"))
    (:NewEnumerator2
      (Collision|SetCollisionEnabled _backunlock "QueryAndPhysics"))
    (:NewEnumerator3
      (Collision|SetCollisionEnabled _backunlock "QueryAndPhysics")
      (Collision|SetCollisionEnabled _frontunlock "QueryAndPhysics")))
  (if (Variables|Default|GetIsAcidDoor?)
    (Rendering|SetVisibility (Variables|Default|GetSlime) true false)))
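; BP_HangarDoor is an interactable hangar door that opens for a player carrying a keycard and leads to the End_Survive level.
; On interaction it checks the player's inventory slots for a single-keycard entry, switches its box collision to overlap and plays the opening montage on the skeletal mesh.
; When the montage completes, it restores blocking collision and loads End_Survive.
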(event Custom|OnInteractWith
  (params (Player :type CH%20Player%20Object%20Reference))
  (bind _box (Variables|Default|GetBox))
  (if (Utilities|Array|ContainsItem (Variables|/Game/GameStuff/Blueprints/Inventory/BP_Inventory.BP_Inventory_C|GetSlots (Variables|/Game/GameStuff/Blueprints/Characters/CH_Player.CH_Player_C|GetInventory Player)) (Utilities|Struct|MakeS_InventorySlot "/Game/GameStuff/Blueprints/Inventory/Items/Item_Keycard.Item_Keycard_C" 1))
    (Collision|SetCollisionProfileName _box "OverlapAllDynamic" :!class /Script/Engine.PrimitiveComponent)
    (Animation|Montage|PlayMontage (Variables|Default|GetSkeletalMesh) "/Game/GameStuff/Models/Doors/Hangar/Animations/Hangar_Opening_Montage.Hangar_Opening_Montage"
      (:OnCompleted
        (Collision|SetCollisionProfileName _box "BlockAll" :!class /Script/Engine.PrimitiveComponent)
        (Game|OpenLevel(byName) "End_Survive")))))

(event EventBeginPlay)

(event Collision|EventActorBeginOverlap
  (params (OtherActor :type Actor%20Object%20Reference)))

(event EventTick
  (params (DeltaSeconds :type Float%20%28single-precision%29)))

(fn ConstructionScript)
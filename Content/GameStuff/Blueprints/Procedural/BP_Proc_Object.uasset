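; Procedural spline placement actor that scatters meshes along its spline at construction time, with no active runtime logic.
; For each ProcData entry, it adds a Hierarchical Instanced Static Mesh component and steps along the spline at that entry's spacing.
; PlaceMesh adds each instance with a world-space offset and random per-axis scale.
; Helper components WS and LS compose spline rotation with the rotation offset, and AlignToZ keeps only yaw.
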(event EventBeginPlay)

(event Collision|EventActorBeginOverlap
  (params (OtherActor :type Actor%20Object%20Reference)))

(event EventTick
  (params (DeltaSeconds :type Float%20%28single-precision%29)))

(fn ConstructionScript
  (for _array_element (Variables|Default|GetProcData)
    (bind _returnvalue (AddComponent|AddHierarchicalInstancedStaticMeshComponent false))
    (bind _output_get (Variables|Default|SetHISM_Current _returnvalue))
    (Components|StaticMesh|SetStaticMesh _output_get (.Mesh (Utilities|Struct|BreakS_ProcElements _array_element)))
    (Variables|Default|SetPlacingDistance 0.0)
    (Utilities|PlaceMesh (Variables|Default|GetPlacingDistance) (.Offset (Utilities|Struct|BreakS_ProcElements _array_element)) (.RotationOffset (Utilities|Struct|BreakS_ProcElements _array_element)) (.ScaleMin (Utilities|Struct|BreakS_ProcElements _array_element)) (.ScaleMax (Utilities|Struct|BreakS_ProcElements _array_element)) (.AlignToZ? (Utilities|Struct|BreakS_ProcElements _array_element)) :!label _label
      (:OUT
        (Variables|Default|SetPlacingDistance (+ (Variables|Default|GetPlacingDistance) (.Distance (Utilities|Struct|BreakS_ProcElements _array_element))))
        (if (< (Variables|Default|GetPlacingDistance) (Spline|GetSplineLength (Variables|Default|GetSpline)))
          (goto _label))))))